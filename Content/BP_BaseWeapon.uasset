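; Base weapon actor that acts as an interactable object in the world.
; On overlap begin and end, it registers or unregisters itself with the other actor's InteractorComponent.
; Focus events toggle a highlight on its skeletal mesh and print debug messages, while the Interaction event is left empty.
; Getter functions expose the center of mass and the skeletal mesh as the interactable mesh.
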(event Collision|EventActorEndOverlap
  (params (OtherActor :type Actor%20Object%20Reference))
  (bind _returnvalue (Actor|GetComponentbyClass OtherActor "/Script/Interaction.InteractorComponent"))
  (Utilities|IsValid _returnvalue
    (:Is%20Valid
      (Class|InteractorComponent|UnregisterInteraction _returnvalue self))))

(event EventOnFocus
  (Class|HighlightComponent|SetHighlight (Variables|Default|GetHighlight) (Variables|Default|GetSkeletalMesh))
  (Development|PrintString "I'm On"))

(event EventOffFocus
  (Class|HighlightComponent|UnsetHighlight (Variables|Default|GetHighlight) (Variables|Default|GetSkeletalMesh))
  (Development|PrintString "I'm Off"))

(event Collision|EventActorBeginOverlap
  (params (OtherActor :type Actor%20Object%20Reference))
  (bind _returnvalue (Actor|GetComponentbyClass OtherActor "/Script/Interaction.InteractorComponent"))
  (Utilities|IsValid _returnvalue
    (:Is%20Valid
      (Class|InteractorComponent|RegisterInteraction _returnvalue self))))

(event EventInteraction)

(fn ConstructionScript)

(fn GetCenterOfMass
  (bind _returnvalue (Class|Interactable|GetCenterOfMass))
  (return _returnvalue))

(fn GetInteractableMesh
  (return (Variables|Default|GetSkeletalMesh)))