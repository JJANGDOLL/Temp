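; Base interactable actor that registers itself with an overlapping actor's InteractorComponent and unregisters when the overlap ends.
; Focus events toggle a Highlight on the static mesh, falling back to the skeletal mesh and printing an error if neither is set.
; The Interaction event only prints a placeholder message, and GetCenterOfMass returns the Sphere's center of mass.
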(event Collision|EventActorEndOverlap
  (params (OtherActor :type Actor%20Object%20Reference))
  (bind _returnvalue (Actor|GetComponentbyClass OtherActor "/Script/Interaction.InteractorComponent"))
  (Utilities|IsValid _returnvalue
    (:Is%20Valid
      (Class|InteractorComponent|UnregisterInteraction _returnvalue self))))

(event EventOnFocus
  (bind _staticmesh (Variables|Default|GetStaticMesh))
  (bind _highlight (Variables|Default|GetHighlight))
  (bind _skeletalmesh (Variables|Default|GetSkeletalMesh))
  (if (!= (Variables|/Script/Engine.StaticMeshComponent|GetStaticMesh _staticmesh) 0)
    (Class|HighlightComponent|SetHighlight _highlight _staticmesh)
    (elif (!= (Variables|/Script/Engine.SkinnedMeshComponent|GetSkeletalMesh _skeletalmesh) 0)
      (Class|HighlightComponent|SetHighlight _highlight _skeletalmesh)
      (else
        (Development|PrintString "Mesh Error")))))

(event EventOffFocus
  (bind _staticmesh (Variables|Default|GetStaticMesh))
  (bind _skeletalmesh (Variables|Default|GetSkeletalMesh))
  (bind _highlight (Variables|Default|GetHighlight))
  (if (!= (Variables|/Script/Engine.StaticMeshComponent|GetStaticMesh _staticmesh) 0)
    (Class|HighlightComponent|UnsetHighlight _highlight _staticmesh)
    (elif (!= (Variables|/Script/Engine.SkinnedMeshComponent|GetSkeletalMesh _skeletalmesh) 0)
      (Class|HighlightComponent|UnsetHighlight _highlight _skeletalmesh)
      (else
        (Development|PrintString "Mesh Error")))))

(event Collision|EventActorBeginOverlap
  (params (OtherActor :type Actor%20Object%20Reference))
  (bind _returnvalue (Actor|GetComponentbyClass OtherActor "/Script/Interaction.InteractorComponent"))
  (Utilities|IsValid _returnvalue
    (:Is%20Valid
      (Class|InteractorComponent|RegisterInteraction _returnvalue self))))

(event EventInteraction
  (Development|PrintString "Base Interaction Called"))

(fn ConstructionScript)

(fn GetCenterOfMass
  (return (Physics|GetCenterOfMass (Variables|Default|GetSphere) "None")))