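; BP_Weapon1 is an interactable weapon item, currently a placeholder whose interaction only prints its name.
; It exposes its StaticMesh as the interactable mesh and returns its ItemInfo through getter functions.
; The center of mass getter returns a zero vector, and SetItemInfo is an empty stub.
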(event EventBeginPlay)

(event Collision|EventActorBeginOverlap
  (params (OtherActor :type Actor%20Object%20Reference))
  (|CallParentFunction OtherActor) ; This node is disabled and will not be called.\nDrag off pins to build functionality.
)

(event EventInteraction
  (Development|PrintString "Weapon1"))

(fn ConstructionScript
  (|CallParentFunction))

(fn GetInteractableMesh
  (return (Variables|Default|GetStaticMesh)))

(fn GetCenterOfMass
  (return "0, 0, 0"))

(fn GetItemInfo
  (return (Variables|Default|GetItemInfo)))

(fn SetItemInfo
  (return))